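; BP_UnitSpawner spawns card-based BP_TestUnit actors once, when something overlaps its Sphere.
; BeginPlay builds a unit pool from DT_Cards using Alignment or Element.
; Spawning places random pool picks at nearby reachable points, plus fixed legend cards for Alignment and Alignment2 when flagged.
; A looping timer destroys the spawner whenever SpawnedUnits is empty, even before triggering, and opens Deckbuilding_Level if it is the last spawner.
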(event `Destroy`
  (if (not (`KismetArrayLibrary.Array_IsValidIndex` (`self.SpawnedUnits`)))
    (bind _outactors (`GameplayStatics.GetAllActorsOfClass` "BP_UnitSpawner_C"))
    (if (<= (`KismetArrayLibrary.Array_Length` _outactors) 1)
      (`GameplayStatics.OpenLevel` "Deckbuilding_Level"))
    (`self.K2_DestroyActor`)))

(event `self.ReceiveBeginPlay`
  (if (`self.IsAlignment?`)
    (set `self.CardNames` (select `/Game/CardStuff/ENUM_ST_DT/Enums/TypeAlignment_Enum` (`self.Alignment`) :!type "Array of Name"))
    (else
      (set `self.CardNames` (select `/Game/CardStuff/ENUM_ST_DT/Enums/ElementalAlignment_Enum` (`self.Element`) :`NewEnumerator0` (`self.Force`) :`NewEnumerator10` (`self.Dark`) :`NewEnumerator9` (`self.Light`) :`NewEnumerator3` (`self.Water`) :`NewEnumerator1` (`self.Fire`) :`NewEnumerator4` (`self.Air`) :`NewEnumerator2` (`self.Earth`)))))
  (`KismetSystemLibrary.K2_SetTimerDelegate` (delegate `Destroy`) 10.0 true)
  (for _array_element (`self.CardNames`)
    (bind _returnvalue (`|GetDataTableRow` "/Game/CardStuff/ENUM_ST_DT/DataTables/DT_Cards.DT_Cards" _array_element)
      (:`then`
        (`KismetArrayLibrary.Array_AddUnique` (`self.PossibleUnits`) _returnvalue)))))

(event `SpawnUnits`
  (bind _lifespan (`self.Lifespan`))
  (bind _lifespan_2 (`self.Lifespan`))
  (bind _lifespan_3 (`self.Lifespan`))
  (if (not (`self.Spawned`))
    (set `self.Spawned` true)
    (for _ (range (+ (`self.Unit#Cap`) 1))
      (bind _returnvalue (`|SpawnActorFromClass` "/Game/BP_TestUnit_Auto2.BP_TestUnit_C" (`KismetMathLibrary.MakeTransform` (`NavigationSystemV1.K2_GetRandomReachablePointInRadius` (`self.K2_GetActorLocation`) 250.0 null null)) "Undefined" "MultiplyWithRoot" null "NewEnumerator4" _lifespan _lifespan (`KismetArrayLibrary.Array_Random` (`self.PossibleUnits`)) null))
      (`KismetArrayLibrary.Array_Add` (`self.SpawnedUnits`) _returnvalue))
    (if (and (`self.IsAlignment?`) (`self.Legend?`))
      (bind _returnvalue_2 (`|GetDataTableRow` "/Game/CardStuff/ENUM_ST_DT/DataTables/DT_Cards.DT_Cards" (select `/Game/CardStuff/ENUM_ST_DT/Enums/TypeAlignment_Enum` (`self.Alignment`) :`NewEnumerator21` "005" :`NewEnumerator0` "040" :`NewEnumerator1` "038" :`NewEnumerator2` "031" :`NewEnumerator4` "024" :!type "Name"))
        (:`then`
          (`|SpawnActorFromClass` "/Game/BP_TestUnit_Auto2.BP_TestUnit_C" (`KismetMathLibrary.MakeTransform` (0.0 0.0 0.0)) "Undefined" "MultiplyWithRoot" null "NewEnumerator4" _lifespan_2 _lifespan_2 _returnvalue_2 null)
          (bind _returnvalue_3 (`|GetDataTableRow` "/Game/CardStuff/ENUM_ST_DT/DataTables/DT_Cards.DT_Cards" (select `/Game/CardStuff/ENUM_ST_DT/Enums/TypeAlignment_Enum` (`self.Alignment2`) :`NewEnumerator21` "005" :`NewEnumerator0` "040" :`NewEnumerator1` "038" :`NewEnumerator2` "031" :`NewEnumerator4` "024" :!type "Name"))
            (:`then`
              (`|SpawnActorFromClass` "/Game/BP_TestUnit_Auto2.BP_TestUnit_C" (`KismetMathLibrary.MakeTransform` (0.0 0.0 0.0)) "Undefined" "MultiplyWithRoot" null "NewEnumerator4" _lifespan_3 _lifespan_3 _returnvalue_3 null))))))))

(event `self.Sphere.OnComponentBeginOverlap`
  (params (OverlappedComponent :type "PrimitiveComponent Object Reference") (OtherActor :type "Actor Object Reference") (OtherComp :type "PrimitiveComponent Object Reference") (OtherBodyIndex :type Integer) (bFromSweep :type Boolean) (SweepResult :type "HitResult Structure (by ref)"))
  (`self.SpawnUnits`))

(fn `UserConstructionScript`)