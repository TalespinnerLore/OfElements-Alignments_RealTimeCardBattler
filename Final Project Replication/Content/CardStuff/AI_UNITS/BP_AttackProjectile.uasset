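; BP_AttackProjectile is a lobbed attack projectile aimed at a target location, with a sphere mesh that takes an element material.
; On BeginPlay it computes a toss velocity with SuggestProjectileVelocity, full-path trace and debug drawing on, and applies it in local space to ProjectileMovement.
; Overlapping any actor without its TeamID tag sends an AttackTargetActor message to the instigator's controller and destroys the projectile.
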(event `self.ReceiveBeginPlay`
  (bind _tossvelocity (`GameplayStatics.BlueprintSuggestProjectileVelocity` (`self.K2_GetActorLocation`) (`self.TargetLocation`) (`self.Speed`) 0.0 "TraceFullPath" 12.5 false true))
  (`ProjectileMovementComponent.SetVelocityInLocalSpace` (`self.ProjectileMovement`) _tossvelocity)
  (`PrimitiveComponent.SetMaterial` (`self.Sphere`) 0 (`self.ElemMaterial`)))

(event `self.ReceiveActorBeginOverlap`
  (params (OtherActor :type "Actor Object Reference"))
  (if (not (`self.ActorHasTag` OtherActor (`KismetStringLibrary.Conv_StringToName` (`|GetEnumeratorNameAsString` (`self.TeamID`)))))
    (message `/Game/CardStuff/AI_UNITS/BPI_COMBAT.AttackTargetActor` (`self.GetInstigatorController`) OtherActor)
    (`self.K2_DestroyActor`)))

(fn `UserConstructionScript`
  (`PrimitiveComponent.SetMaterial` (`self.Sphere`) 0 (`self.ElemMaterial`)))