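; Short-lived area spell actor that applies damage or healing, status changes and spell-specific effects to actors overlapping it.
; Construction selects the mesh by spell shape and sets the element material, while a looping timer counts down to destruction.
; Overlaps are filtered by team tag, healing is negative damage, and statuses come from DT_SpellStatus.
; An element effectiveness function multiplies type-chart lookups but is not called here.
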(event `self.ReceiveBeginPlay`
  (`KismetSystemLibrary.K2_SetTimerDelegate` (delegate `Loop`) (`self.LoopInterval`) true)
  (`self.GetStatusToApply` (`self.SpellEnum`)))

(event `Loop`
  (bind _output_get (set `self.Lifespan` (- (`self.Lifespan`) (`self.LoopInterval`))))
  (if (<= _output_get 0.0)
    (`self.K2_DestroyActor`)))

(event `self.ReceiveActorBeginOverlap`
  (params (OtherActor :type "Actor Object Reference"))
  (bind _returnvalue (`KismetStringLibrary.Conv_StringToName` (`|GetEnumeratorNameAsString` (`self.TeamID`))))
  (switch `/Game/CardStuff/ENUM_ST_DT/Enums/SpellTargetEnum` (`self.LegalTarget`)
    (:`NewEnumerator2`
      (`self.Do Contact Effect` OtherActor (`self.Buff/ Debuff`) (`self.Persistent?`) (`self.Healing`) :!label _label))
    (:`NewEnumerator0`
      (if (not (`self.ActorHasTag` OtherActor _returnvalue))
        (goto _label)))
    (:`NewEnumerator1`
      (if (`self.ActorHasTag` OtherActor _returnvalue)
        (goto _label)))))

(fn `Do Contact Effect`
  (params (TouchedActor :type "Actor Object Reference") (`Buff/Debuff` :type Boolean) (`Persistent?` :type Boolean) (Healing :type Boolean))
  (locals (HealingMultiplier :type "Float (double-precision)" :default 1.0))
  (bind _statustoapply (`self.StatusToApply`))
  (`|ExecutionSequence`
    (:`then_0`
      (if Healing
        (set `local.HealingMultiplier` -1.0)
        (else
          (set `local.HealingMultiplier` 1.0)))
      (`GameplayStatics.ApplyDamage` TouchedActor (* (`local.HealingMultiplier`) (`self.Damage`)) (`self.GetInstigatorController`) self))
    (:`then_1`
      (if `Buff/Debuff`
        (bind _keys (`BlueprintMapLibrary.Map_Keys` _statustoapply))
        (bind _values (`BlueprintMapLibrary.Map_Values` _statustoapply))
        (for (_array_element _array_index) _keys
          (message `/Game/CardStuff/AI_UNITS/BPI_COMBAT.ApplyStatusChange` TouchedActor `Persistent?` _array_element (`KismetMathLibrary.Conv_IntToDouble` (`|GetArrayItem` _values _array_index))))))
    (:`then_2`
      (message `/Game/CardStuff/AI_UNITS/BPI_COMBAT.ApplySpellEffect` TouchedActor (`self.SpellEnum`)))))

(fn `Do Other Effect`)

(fn `ElementEffectiveness`
  (params (AttackElem1 :type "/Game/CardStuff/ENUM_ST_DT/Enums/ElementalAlignment_Enum Enum" :default "NewEnumerator11") (AttackElem2 :type "/Game/CardStuff/ENUM_ST_DT/Enums/ElementalAlignment_Enum Enum" :default "NewEnumerator11") (DefendingElem1 :type "/Game/CardStuff/ENUM_ST_DT/Enums/ElementalAlignment_Enum Enum" :default "NewEnumerator11") (DefendingElem2 :type "/Game/CardStuff/ENUM_ST_DT/Enums/ElementalAlignment_Enum Enum" :default "NewEnumerator11"))
  (returns (EffectivenessMultiplier :type "Float (double-precision)"))
  (locals (Multiplier1 :type "Float (double-precision)" :default 1.0) (Multiplier2 :type "Float (double-precision)" :default 1.0) (Multiplier3 :type "Float (double-precision)" :default 1.0) (Multiplier4 :type "Float (double-precision)" :default 1.0) (AttackElem :type "/Game/CardStuff/ENUM_ST_DT/Enums/ElementalAlignment_Enum Enum" :default "NewEnumerator11") (DefendingElem :type "/Game/CardStuff/ENUM_ST_DT/Enums/ElementalAlignment_Enum Enum") (Counter :type Integer) (FinalMultiplier :type "Float (double-precision)"))
  (set `local.Counter` 1)
  (`|ExecutionSequence`
    (:`then_0`
      (set `local.AttackElem` AttackElem1)
      (set `local.DefendingElem` DefendingElem1))
    (:`then_1`
      (set `local.AttackElem` AttackElem1)
      (set `local.DefendingElem` DefendingElem2)
      (set `local.Counter` 2))
    (:`then_2`
      (set `local.AttackElem` AttackElem2)
      (set `local.DefendingElem` DefendingElem1)
      (set `local.Counter` 3))
    (:`then_3`
      (set `local.AttackElem` AttackElem2)
      (set `local.DefendingElem` DefendingElem2)
      (set `local.Counter` 4))
    (:`then_4`
      (bind _output_get (set `local.FinalMultiplier` (* (`local.Multiplier1`) (`local.Multiplier2`) (`local.Multiplier3`) (`local.Multiplier4`))))
      (return _output_get)))
  (bind _returnvalue (`|GetDataTableRow` "/Game/CardStuff/ENUM_ST_DT/DataTables/DT_ElemTypeChart.DT_ElemTypeChart" (`KismetStringLibrary.Conv_StringToName` (`KismetStringLibrary.Conv_ByteToString` (`local.AttackElem`))))
    (:`then`
      _)
    (:`RowNotFound`
      (set `local.DefendingElem` "NewEnumerator11")))
  (switch `int` (`local.Counter`)
    (:`1`
      (bind (_force _dark _light _water _fire _air _earth) (break `/Game/CardStuff/ENUM_ST_DT/Structs/ST_ElementTypeChart` _returnvalue))
      (bind _returnvalue_2 (select `/Game/CardStuff/ENUM_ST_DT/Enums/ElementalAlignment_Enum` (`local.DefendingElem`) :`NewEnumerator11` 1.0 :`NewEnumerator0` _force :`NewEnumerator10` _dark :`NewEnumerator9` _light :`NewEnumerator3` _water :`NewEnumerator1` _fire :`NewEnumerator4` _air :`NewEnumerator2` _earth))
      (set `local.Multiplier1` _returnvalue_2))
    (:`2`
      (set `local.Multiplier2` _returnvalue_2))
    (:`3`
      (set `local.Multiplier3` _returnvalue_2))
    (:`4`
      (set `local.Multiplier4` _returnvalue_2))))

(fn `GetStatusToApply`
  (params (SpellEnum :type "/Game/CardStuff/ENUM_ST_DT/Enums/SpellEffect_Enum Enum" :default "NewEnumerator0"))
  (bind _returnvalue (`|GetDataTableRow` "/Game/CardStuff/ENUM_ST_DT/DataTables/DT_SpellStatus.DT_SpellStatus" (`KismetStringLibrary.Conv_StringToName` (`|GetEnumeratorNameAsString` SpellEnum)))
    (:`then`
      (set `self.StatusToApply` (`.StatusEffects_9_2DAE59294DDD2FB942B3B19A5CE68E3C` (break `/Game/CardStuff/ENUM_ST_DT/Structs/ST_SpellStatus` _returnvalue))))))

(fn `UserConstructionScript`
  (bind _aoe (`self.AoE`))
  (`StaticMeshComponent.SetStaticMesh` _aoe (select `/Game/CardStuff/ENUM_ST_DT/Enums/SpellShape_Enum` (`self.SpellShape`) :`NewEnumerator0` "/Game/UnrealContent/Cursor/SM_CursorMesh.SM_CursorMesh" :`NewEnumerator1` "/Game/CardStuff/AI_UNITS/SpellShape_Circle.SpellShape_Circle" :`NewEnumerator2` "/Game/CardStuff/AI_UNITS/SpellShape_Cone.SpellShape_Cone" :`NewEnumerator3` "/Game/CardStuff/AI_UNITS/SpellShape_Line.SpellShape_Line" :!type "StaticMesh Object Reference"))
  (`PrimitiveComponent.SetMaterial` _aoe 0 (`self.ElemMaterial`)))