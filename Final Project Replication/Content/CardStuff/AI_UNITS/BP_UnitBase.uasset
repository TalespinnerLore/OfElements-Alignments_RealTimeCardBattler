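; BP_UnitBase is the base Blueprint for card-spawned AI units, which live on the field for a limited duration.
; Construction sets the mesh and multi-element flag from UnitStats, and BeginPlay caches the indicator widget and combat controller.
; A looping timer updates the indicator's countdown, then on expiry has the controller check resources, returns the card to the deck bottom and destroys the unit.
; RandomRoam, uncalled here, repeatedly moves toward the player.
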(event `RandomRoam`
  (`|AIMoveTo` self (0.0 0.0 0.0) (`GameplayStatics.GetPlayerCharacter` 0) 1.0 true
    (:`then`
      (`KismetSystemLibrary.PrintString` "roaming"))
    (:`OnSuccess`
      (`KismetSystemLibrary.Delay` (`KismetMathLibrary.RandomFloatInRange` 0.0 0.2))
      (`KismetSystemLibrary.PrintString` "roamed")
      (`self.RandomRoam`))))

(event `self.ReceiveBeginPlay`
  (`KismetSystemLibrary.K2_SetTimerDelegate` (delegate `Timer`) (`self.Interval`) true)
  (set `self.Timer Duration` (`.DurationMultiplier_116_D49F686C4944CF75721284A4F87F1FF3` (break `/Game/CardStuff/ENUM_ST_DT/Structs/AllCardStats_Struct` (`self.UnitStats`))))
  (bind _aswbp_unit_indicators (cast `/Game/CardStuff/UI/CombatUI/WBP_UnitIndicators` (`WidgetComponent.GetUserWidgetObject` (`self.Widget`)))
    (:`then`
      (bind _output_get (set `self.Unit Indicators` _aswbp_unit_indicators))
      (`/Game/CardStuff/UI/CombatUI/WBP_UnitIndicators.SetAlignment/Element` _output_get "/Game/CardStuff/TEXTURES/CardTextures/Element_Alignment_Icons/ForceIcon.ForceIcon" "/Game/CardStuff/TEXTURES/CardTextures/Element_Alignment_Icons/ForceIcon.ForceIcon")
      (bind _asbp_combat_controller_new (cast `/Game/CardStuff/PLAYER/BP_CombatController_New` (`GameplayStatics.GetPlayerController` 0)))
      (bind _output_get_2 (set `self.ControllerRef` _asbp_combat_controller_new))
      (`KismetSystemLibrary.PrintString` (`KismetSystemLibrary.GetDisplayName` _output_get_2) true true (struct :`R` 1.0 :`G` 0.716424 :`A` 1.0)))
    (:`CastFailed`
      (`KismetSystemLibrary.PrintString` "BAD INDICATOR"))))

(event `Timer`
  (bind _controllerref (`self.ControllerRef`))
  (bind _output_get (set `self.Timer Duration` (- (`self.Timer Duration`) (`self.Interval`))))
  (`/Game/CardStuff/UI/CombatUI/WBP_UnitIndicators.TimerPercent` (`self.Unit Indicators`) (/ _output_get (`.DurationMultiplier_116_D49F686C4944CF75721284A4F87F1FF3` (break `/Game/CardStuff/ENUM_ST_DT/Structs/AllCardStats_Struct` (`self.UnitStats`)))))
  (if (<= (`self.Timer Duration`) 0.0)
    (`/Game/CardStuff/PLAYER/BP_CombatController_New.CheckResoucePastMax` _controllerref)
    (`/Game/CardStuff/PLAYER/BP_DeckBearer_Char.FieldToDeck[Bottom]` (`/Game/CardStuff/PLAYER/BP_CombatController_New.PlayerRef` _controllerref) (`self.UnitStats`))
    (`self.K2_DestroyActor`)))

(fn `Return Cost`
  (locals (PrimaryResource :type Integer :default 0) (SecondaryResource :type Integer :default 0) (Cost :type Integer)))

(fn `UserConstructionScript`
  (bind (_name _unique_ _cost _primaryalignment _secondaryalignment _primaryelement _secondaryelement _durationmultiplier _cardtype _creaturestats _spellstats _targeting _triggers _mesh) (break `/Game/CardStuff/ENUM_ST_DT/Structs/AllCardStats_Struct` (`self.UnitStats`)))
  (`StaticMeshComponent.SetStaticMesh` (`self.Cube`) _mesh)
  (set `self.MultiElement?` (`|EnumInequality` _secondaryalignment "NewEnumerator22")))