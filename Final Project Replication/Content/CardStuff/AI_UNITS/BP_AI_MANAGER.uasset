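; BP_AI_MANAGER holds the card game's global effects and checks units or cards against them, despite its AI manager name.
; CheckGlobals matches enabled effects by zone, returning a discount for Hand on an element match.
; For Field, an element or alignment match permanently applies the effect's buff and debuff statuses to the unit.
; StartEndEffect sets effects' Enabled flag by ID; the event graph holds only disabled or unwired nodes.
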(fn `CheckGlobals`
  (params (ZoneToCheck :type "/Game/CardStuff/ENUM_ST_DT/Enums/Zone_Enum Enum" :default "NewEnumerator0") (Alignment1 :type "/Game/CardStuff/ENUM_ST_DT/Enums/TypeAlignment_Enum Enum" :default "NewEnumerator21") (Alignment2 :type "/Game/CardStuff/ENUM_ST_DT/Enums/TypeAlignment_Enum Enum" :default "NewEnumerator21") (Elem1 :type "/Game/CardStuff/ENUM_ST_DT/Enums/ElementalAlignment_Enum Enum" :default "NewEnumerator11") (Elem2 :type "/Game/CardStuff/ENUM_ST_DT/Enums/ElementalAlignment_Enum Enum" :default "NewEnumerator11") (Unit :type "/Game/BP_TestUnit_Auto2 Object Reference"))
  (returns (Discount :type Integer))
  (set `self.Zone to Check` ZoneToCheck)
  (set `self.Alignment 1` Alignment1)
  (set `self.Alignment 2` Alignment2)
  (set `self.Elem 1` Elem1)
  (set `self.Elem 2` Elem2)
  (for _array_element (`self.GlobalEffects`)
    (bind (_effectid _cardtype _enabled_ _affected_teamid _affected_zone _affected_alignment _affected_element _buff_ _debuff_ _discount_) (break `/Game/CardStuff/ENUM_ST_DT/Structs/ST_GlobalEffects` _array_element))
    (if (and (`|EnumEquality` (`self.Zone to Check`) _affected_zone) _enabled_)
      (switch `/Game/CardStuff/ENUM_ST_DT/Enums/Zone_Enum` _affected_zone
        (:`NewEnumerator0`
          (bind _returnvalue (or (`|EnumEquality` _affected_element (`self.Elem 2`)) (`|EnumEquality` (`self.Elem 1`) _affected_element)))
          (if _returnvalue
            (return _discount_)))
        (:`NewEnumerator2`
          (if (or (or (`|EnumEquality` _affected_alignment (`self.Alignment 2`)) (`|EnumEquality` (`self.Alignment 1`) _affected_alignment)) _returnvalue)
            (bind _values (`BlueprintMapLibrary.Map_Values` _buff_))
            (bind _keys (`BlueprintMapLibrary.Map_Keys` _buff_))
            (for (_array_element_2 _array_index) _keys
              (message `/Game/CardStuff/AI_UNITS/BPI_COMBAT.ApplyStatusChange` (`local.Unit`) true _array_element_2 (`KismetMathLibrary.Conv_IntToDouble` (`|GetArrayItem` _values _array_index))))
            (bind _values_2 (`BlueprintMapLibrary.Map_Values` _debuff_))
            (bind _keys_2 (`BlueprintMapLibrary.Map_Keys` _debuff_))
            (for (_array_element_3 _array_index_2) _keys_2
              (message `/Game/CardStuff/AI_UNITS/BPI_COMBAT.ApplyStatusChange` (`local.Unit`) true _array_element_3 (`KismetMathLibrary.Conv_IntToDouble` (`|GetArrayItem` _values_2 _array_index_2))))))))))

(fn `Start/EndEffect`
  (params (EffectID :type "/Game/CardStuff/ENUM_ST_DT/Enums/GlobalEffects_Enum Enum" :default "NewEnumerator0") (`Starting?` :type Boolean))
  (for _array_element (`self.GlobalEffects`)
    (if (`|EnumEquality` EffectID (`.EffectID_31_BDAC0F1E488AF794DE974D95CF6F2B1E` (break `/Game/CardStuff/ENUM_ST_DT/Structs/ST_GlobalEffects` _array_element)))
      (setmembers `/Game/CardStuff/ENUM_ST_DT/Structs/ST_GlobalEffects` :`StructRef` _array_element :`Enabled?` `Starting?`))))

(fn `UserConstructionScript`)