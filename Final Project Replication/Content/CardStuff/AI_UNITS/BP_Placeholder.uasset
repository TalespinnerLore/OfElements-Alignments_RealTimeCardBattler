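; Cursor-following placement preview for a card being played, showing either a creature mesh or a spell area shape.
; A looping timer moves it to the cursor ray projected onto Z=0, or rotates player-fixed spells toward the cursor.
; Materials show validity from hand range, plus overlaps for creatures.
; Spell-area overlaps outline team-filtered targets through custom depth; an older SpellTick remains unused.
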(event `SpellTick`
  (bind _aoe (`self.AoE`))
  (bind (_singletarget_ _targetactor _friendlyfire_ _targetlocation _aoetype _radius) (break `/Game/CardStuff/ENUM_ST_DT/Structs/TargetingStruct` (`.Targeting_107_6D44DCD64434A8C803037998A6E7DFDC` (break `/Game/CardStuff/ENUM_ST_DT/Structs/AllCardStats_Struct` (`/Game/CardStuff/UI/CombatUI/WBP_CardInHand.CardStats` (`self.OriginCard`))))))
  (bind _returnvalue (< (`KismetMathLibrary.Vector_Distance` (`self.K2_GetActorLocation` (`GameplayStatics.GetPlayerCharacter` 0)) (`self.K2_GetActorLocation`)) (`self.Char-Hand Distance`)))
  (if (`self.WasRecentlyRendered` 0.02)
    (`self.K2_SetActorLocation` (`self.LocationUnderCursor`))
    (if _singletarget_
      (bind _output_get (set `self.TargetActor` (`|GetArrayItem` (`self.GetOverlappingActors` _targetactor))))
      (bind _output_get_2 (set `self.ValidTarget` (and (`KismetSystemLibrary.IsValid` _output_get) _returnvalue)))
      (`PrimitiveComponent.SetMaterial` (`self.Sphere`) 0 (select `bool` _output_get_2 :`false` "/Game/UnrealContent/StarterContent/Particles/Materials/M_explosion_subUV.M_explosion_subUV" :`true` "/Game/UnrealContent/StarterContent/Particles/Materials/M_smoke_subUV.M_smoke_subUV" :!type "MaterialInterface Object Reference"))
      (else
        (`SceneComponent.SetVisibility` _aoe true false)
        (`SceneComponent.SetRelativeScale3D` _aoe (`KismetMathLibrary.Conv_DoubleToVector` _radius))
        (`StaticMeshComponent.SetStaticMesh` _aoe (select `/Game/CardStuff/ENUM_ST_DT/Enums/AoE_Type_Enum` _aoetype :`NewEnumerator0` "/Game/UnrealContent/StarterContent/Shapes/Shape_Cylinder.Shape_Cylinder" :`NewEnumerator1` "/Game/UnrealContent/StarterContent/Shapes/Shape_Wedge_A.Shape_Wedge_A" :`NewEnumerator2` "/Game/UnrealContent/StarterContent/Shapes/Shape_Pipe.Shape_Pipe" :!type "StaticMesh Object Reference"))
        (bind _output_get_3 (set `self.ValidTarget` (and (== (`KismetArrayLibrary.Array_Length` (`PrimitiveComponent.GetOverlappingActors` (`self.Sphere`) "/Game/CardStuff/SINGLEPLAYER/BP_BlockGrid.BP_BlockGrid_C")) 0) _returnvalue)))
        (bind _returnvalue_2 (select `bool` _output_get_3 :`false` "/Game/UnrealContent/StarterContent/Particles/Materials/M_explosion_subUV.M_explosion_subUV" :`true` "/Game/UnrealContent/StarterContent/Particles/Materials/M_smoke_subUV.M_smoke_subUV" :!type "MaterialInterface Object Reference"))
        (`PrimitiveComponent.SetMaterial` (`self.Sphere`) 0 _returnvalue_2)
        (`PrimitiveComponent.SetMaterial` (`self.AoE`) 0 _returnvalue_2)))
    (else
      (`KismetSystemLibrary.PrintString` "GEK" true true (struct :`R` 1.0 :`G` 0.152253 :`A` 1.0))
      (`self.K2_DestroyActor`))))

(event `ClearTimers`
  (`KismetSystemLibrary.K2_ClearTimer` null "SpellTick")
  (`KismetSystemLibrary.K2_ClearTimer` null "CreatureTick"))

(event `CreatureTick`
  (if (`self.WasRecentlyRendered` 0.02)
    (`self.K2_SetActorLocation` (`self.LocationUnderCursor`))
    (set `self.Placeable?` (and (== (`KismetArrayLibrary.Array_Length` (`self.GetOverlappingActors` null)) 0) (< (`KismetMathLibrary.Vector_Distance` (`self.K2_GetActorLocation` (`GameplayStatics.GetPlayerCharacter` 0)) (`self.K2_GetActorLocation`)) (`self.Char-Hand Distance`))))
    (`PrimitiveComponent.SetMaterial` (`self.Sphere`) 0 (select `bool` (`self.Placeable?`) :`false` "/Game/CardStuff/MATERIALS/M_Invalid.M_Invalid" :`true` "/Game/CardStuff/MATERIALS/M_Valid.M_Valid" :!type "MaterialInterface Object Reference"))
    (else
      (`KismetSystemLibrary.PrintString` "GEK" true true (struct :`R` 1.0 :`G` 0.152253 :`A` 1.0))
      (`self.K2_DestroyActor`))))

(event `self.ReceiveBeginPlay`
  (bind (_fixedtoplayer_ _traveltype _spellshape _spelleffect _legaltarget _radiuswidth _length) (break `/Game/CardStuff/ENUM_ST_DT/Structs/ST_SpellStats` (`.SpellStats_120_0DE33AA348A0F5684E7101855C1789D7` (break `/Game/CardStuff/ENUM_ST_DT/Structs/AllCardStats_Struct` (`/Game/CardStuff/UI/CombatUI/WBP_CardInHand.CardStats` (`self.OriginCard`))))))
  (switch `/Game/CardStuff/ENUM_ST_DT/Enums/CardType_Enum` (`self.CardType`)
    (:`NewEnumerator0`
      (`KismetSystemLibrary.K2_SetTimerDelegate` (delegate `CreatureTick`) 0.1 true))
    (:`NewEnumerator3`
      (`KismetSystemLibrary.K2_SetTimerDelegate` (delegate `SpellTick(new)`) 0.1 true)
      (`StaticMeshComponent.SetStaticMesh` (`self.AoE`) (select `/Game/CardStuff/ENUM_ST_DT/Enums/SpellShape_Enum` (`self.SpellSHape`) :`NewEnumerator0` "/Game/UnrealContent/StarterContent/Props/MaterialSphere.MaterialSphere" :`NewEnumerator1` "/Game/CardStuff/AI_UNITS/SpellShape_Circle.SpellShape_Circle" :`NewEnumerator2` "/Game/CardStuff/AI_UNITS/SpellShape_Cone.SpellShape_Cone" :`NewEnumerator3` "/Game/CardStuff/AI_UNITS/SpellShape_Line.SpellShape_Line" :!type "StaticMesh Object Reference"))
      (`SceneComponent.SetWorldScale3D` (`self.AoE`) (`KismetMathLibrary.MakeVector` _length _radiuswidth 1.0))
      (`SceneComponent.SetVisibility` (`self.Sphere`) false false)
      (`SceneComponent.SetVisibility` (`self.AoE`) true false))))

(event `SpellTick(new)`
  (bind (_fixedtoplayer_ _traveltype _spellshape _spelleffect _legaltarget) (break `/Game/CardStuff/ENUM_ST_DT/Structs/ST_SpellStats` (`.SpellStats_120_0DE33AA348A0F5684E7101855C1789D7` (break `/Game/CardStuff/ENUM_ST_DT/Structs/AllCardStats_Struct` (`/Game/CardStuff/UI/CombatUI/WBP_CardInHand.CardStats` (`self.OriginCard`))))))
  (bind (_returnvalue_roll _returnvalue_pitch _returnvalue_yaw) (`KismetMathLibrary.BreakRotator` (`KismetMathLibrary.Conv_VectorToRotator` (- (`self.LocationUnderCursor`) (`SceneComponent.K2_GetComponentLocation` (`self.AoE`))))))
  (`self.K2_SetActorLocation` (`self.K2_GetActorLocation` (`GameplayStatics.GetPlayerCharacter` 0)))
  (if _fixedtoplayer_
    (`KismetSystemLibrary.PrintString` (`KismetStringLibrary.Conv_DoubleToString` _returnvalue_yaw))
    (`self.K2_SetActorRotation` (`KismetMathLibrary.MakeRotator` 0.0 0.0 _returnvalue_yaw))
    (else
      (`self.K2_SetActorLocation` (`self.LocationUnderCursor`))))
  (if (`|EnumEquality` _spellshape "NewEnumerator0")
    _
    (else
      _))
  (set `self.Placeable?` (< (`KismetMathLibrary.Vector_Distance` (`self.K2_GetActorLocation` (`GameplayStatics.GetPlayerCharacter` 0)) (`self.K2_GetActorLocation`)) (`self.Char-Hand Distance`)))
  (`PrimitiveComponent.SetMaterial` (`self.AoE`) 0 (select `bool` (`self.Placeable?`) :`false` "/Game/CardStuff/MATERIALS/M_Invalid.M_Invalid" :`true` "/Game/CardStuff/MATERIALS/M_Valid.M_Valid" :!type "MaterialInterface Object Reference")))

(event `self.AoE.OnComponentBeginOverlap`
  (params (OverlappedComponent :type "PrimitiveComponent Object Reference") (OtherActor :type "Actor Object Reference") (OtherComp :type "PrimitiveComponent Object Reference") (OtherBodyIndex :type Integer) (bFromSweep :type Boolean) (SweepResult :type "HitResult Structure (by ref)"))
  (bind _returnvalue (`KismetStringLibrary.Conv_StringToName` (`|GetEnumeratorNameAsString` (`self.TeamID`))))
  (bind (_fixedtoplayer_ _traveltype _spellshape _spelleffect _legaltarget) (break `/Game/CardStuff/ENUM_ST_DT/Structs/ST_SpellStats` (`.SpellStats_120_0DE33AA348A0F5684E7101855C1789D7` (break `/Game/CardStuff/ENUM_ST_DT/Structs/AllCardStats_Struct` (`/Game/CardStuff/UI/CombatUI/WBP_CardInHand.CardStats` (`self.OriginCard`))))))
  (switch `/Game/CardStuff/ENUM_ST_DT/Enums/SpellTargetEnum` _legaltarget
    (:`NewEnumerator2`
      (if (`|EnumEquality` _spellshape "NewEnumerator0") :!label _label
        (for _array_element (`self.K2_GetComponentsByClass` (`self.TargetActor`) "/Script/Engine.MeshComponent")
          (`PrimitiveComponent.SetRenderCustomDepth` _array_element false))
        ;[1 1 1] Outline Affected Actor
        (set `self.TargetActor` OtherActor))
      (for _array_element_2 (`self.K2_GetComponentsByClass` OtherActor "/Script/Engine.MeshComponent")
        (`PrimitiveComponent.SetRenderCustomDepth` _array_element_2 true)
        (set `self.ValidTarget` true)))
    (:`NewEnumerator0`
      (if (not (`self.ActorHasTag` OtherActor _returnvalue))
        (goto _label)))
    (:`NewEnumerator1`
      (if (`self.ActorHasTag` OtherActor _returnvalue)
        (goto _label)))))

(event `self.AoE.OnComponentEndOverlap`
  (params (OverlappedComponent :type "PrimitiveComponent Object Reference") (OtherActor :type "Actor Object Reference") (OtherComp :type "PrimitiveComponent Object Reference") (OtherBodyIndex :type Integer))
  ;[1 1 1] De-Outline Affected Actor
  (if (not (`|EnumEquality` (`.SpellShape_9_C558E84148689EA6EFFDDCA9820B5B90` (break `/Game/CardStuff/ENUM_ST_DT/Structs/ST_SpellStats` (`.SpellStats_120_0DE33AA348A0F5684E7101855C1789D7` (break `/Game/CardStuff/ENUM_ST_DT/Structs/AllCardStats_Struct` (`/Game/CardStuff/UI/CombatUI/WBP_CardInHand.CardStats` (`self.OriginCard`)))))) "NewEnumerator0"))
    (for _array_element (`self.K2_GetComponentsByClass` OtherActor "/Script/Engine.MeshComponent")
      (`PrimitiveComponent.SetRenderCustomDepth` _array_element false)
      (if (<= (`KismetArrayLibrary.Array_Length` (`self.GetOverlappingActors` null)) 0)
        (set `self.ValidTarget` false)))))

(fn `LocationUnderCursor`
  (returns (Location :type "Vector Structure"))
  (locals (UnderCursor :type "Vector Structure") (CameraLoc :type "Vector Structure" :default (0.0 0.0 0.0)))
  (bind _returnvalue (`PlayerCameraManager.GetCameraLocation` (`GameplayStatics.GetPlayerCameraManager` 0)))
  (bind _output_get (set `local.CameraLoc` _returnvalue))
  (bind _output_get_2 (set `local.UnderCursor` (- (`.Location` (`GameplayStatics.BreakHitResult` (`PlayerController.GetHitResultUnderCursorByChannel` (`GameplayStatics.GetPlayerController` 0) "TraceTypeQuery2" true))) _returnvalue)))
  (return (+ (`local.CameraLoc`) (* (`local.UnderCursor`) (/ (.z _output_get) (.z _output_get_2) -1.0)))))

(fn `UserConstructionScript`
  (`StaticMeshComponent.SetStaticMesh` (`self.Sphere`) (`self.InputMesh`)))