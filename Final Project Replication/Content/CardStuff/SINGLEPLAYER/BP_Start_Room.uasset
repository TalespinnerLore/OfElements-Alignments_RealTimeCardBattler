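; Start room that procedurally generates a branching corridor layout on BeginPlay from a fixed-seed random stream.
; Each corridor chains BP_Generator_Path actors with random stepped turns, stopping when a forward sphere trace hits something.
; Random or near-end branch points join the spawn list while the branch budget lasts, seeding further corridors.
; Corridors reaching full length add an end transform, offset forward, to BP_BlockGrid's EndPoints.
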(event `self.ReceiveBeginPlay`
  (set `self.RandomStream` (`KismetMathLibrary.MakeRandomStream` 0))
  (`KismetArrayLibrary.Array_Set` (`self.SpawnPoints`) 0 (`SceneComponent.K2_GetComponentToWorld` (`self.PathStartPoint`)) true)
  (`KismetArrayLibrary.Array_Set` (`self.SpawnPointVectors`) 0 (`SceneComponent.GetForwardVector` (`self.PathStartPoint`)) true)
  (for (_array_element _array_index) (`self.SpawnPoints`)
    (bind _output_get (set `self.CorridorLength` (`KismetMathLibrary.RandomIntegerInRangeFromStream` (`self.RandomStream`) 5 10)))
    (set `self.First` true)
    (`self.SpawnCorridor(s)` _array_element _output_get (`|GetArrayItem` (`self.SpawnPointVectors`) _array_index))))

(fn `CheckInFront`
  (params (Transfrom :type "Transform Structure") (FrontVector :type "Vector Structure") (Transfrom_Location :type "Vector Structure" :default (0.0 0.0 0.0)) (Transfrom_Rotation :type "Rotator Structure" :default (struct)) (Transfrom_Scale :type "Vector Structure" :default (0.0 0.0 0.0)))
  (returns (`Hit?` :type Boolean))
  (bind (_outhits _returnvalue) (`KismetSystemLibrary.SphereTraceMulti` :`Start` (+ Transfrom_Location (* FrontVector 110.0)) :`End` (+ Transfrom_Location (* FrontVector 300.0)) :`Radius` 100.0 :`TraceChannel` "TraceTypeQuery1" :`bTraceComplex` true :`DrawDebugType` "Persistent"))
  (return _returnvalue))

(fn `SpawnCorridor(s)`
  (params (SpawnLoc :type "Transform Structure") (HallLength :type Integer) (ForwardVector :type "Vector Structure"))
  (locals (CorridorRotation :type "Rotator Structure" :default (struct)) (CorridorSpawnLoc :type "Transform Structure") (LoopIndex :type Integer) (NewSpawnPoint :type "SceneComponent Object Reference") (TurnRate :type "Float (double-precision)" :default 25.0) (Front :type "Vector Structure") (PathBlock :type "/Game/CardStuff/SINGLEPLAYER/BP_Generator_Path Object Reference") (NewLocalVar :type Boolean :default false))
  (bind _corridorspawnloc_location (`KismetMathLibrary.BreakTransform` (`local.CorridorSpawnLoc`)))
  (bind _newspawnpoint (`local.NewSpawnPoint`))
  (bind _corridorspawnloc_location_2 (`KismetMathLibrary.BreakTransform` (`local.CorridorSpawnLoc`)))
  (bind _front (`local.Front`))
  (bind _corridorspawnloc (`local.CorridorSpawnLoc`))
  (bind (_returnvalue_location _returnvalue_rotation) (`KismetMathLibrary.BreakTransform` (`SceneComponent.K2_GetComponentToWorld` _newspawnpoint)))
  (bind _returnvalue (/ 90.0 (`local.TurnRate`)))
  (bind _returnvalue_2 (> (`self.BranchesToSpawn#`) 0))
  (bind (_returnvalue_x _returnvalue_y _returnvalue_z) (`KismetMathLibrary.BreakVector` (+ (* (`SceneComponent.GetForwardVector` _newspawnpoint) 350.0) _returnvalue_location)))
  (set `local.CorridorSpawnLoc` SpawnLoc)
  (set `local.Front` ForwardVector)
  (for _index (range (+ HallLength 1))
    (set `local.LoopIndex` _index)
    (bind (_outhits _returnvalue_3) (`KismetSystemLibrary.SphereTraceMulti` (+ _corridorspawnloc_location_2 (* _front 110.0)) (+ _corridorspawnloc_location_2 (* _front 150.0)) 100.0 "TraceTypeQuery1" true))
    (if _returnvalue_3
      (break)
      (else
        (if (`self.First`)
          (set `local.CorridorRotation` (`KismetMathLibrary.MakeRotator` 0.0 0.0 (.yaw (.rotation _corridorspawnloc))))
          (set `self.First` false)
          (else
            (set `local.CorridorRotation` (`KismetMathLibrary.MakeRotator` 0.0 0.0 (+ (.yaw (.rotation _corridorspawnloc)) (* (`local.TurnRate`) (`KismetMathLibrary.RandomIntegerInRangeFromStream` (`self.RandomStream`) (* _returnvalue -1.0) (`KismetMathLibrary.FTrunc` _returnvalue))))))))
        (bind _returnvalue_4 (`|SpawnActorFromClass` "/Game/CardStuff/SINGLEPLAYER/BP_Generator_Path.BP_Generator_Path_C" (`KismetMathLibrary.MakeTransform` _corridorspawnloc_location (`local.CorridorRotation`)) "AlwaysSpawn" "MultiplyWithRoot" null null))
        (set `local.PathBlock` _returnvalue_4)
        (bind _startpoint (`/Game/CardStuff/SINGLEPLAYER/BP_Generator_Path.StartPoint` _returnvalue_4))
        (set `local.NewSpawnPoint` _startpoint)
        (set `local.CorridorSpawnLoc` (`SceneComponent.K2_GetComponentToWorld` _startpoint))
        (set `local.Front` (`SceneComponent.GetForwardVector` (`local.NewSpawnPoint`)))
        (bind _output_get (set `local.NewLocalVar` (`KismetMathLibrary.RandomBoolFromStream` (`self.RandomStream`))))
        (if (or (and (> (`KismetMathLibrary.RandomFloatFromStream` (`self.RandomStream`)) 0.9) _returnvalue_2) (and _returnvalue_2 (== (`local.LoopIndex`) (- (`local.HallLength`) 1))))
          (bind _returnvalue_5 (select `bool` _output_get :`false` (`/Game/CardStuff/SINGLEPLAYER/BP_Generator_Path.BranchLeftPoint` _returnvalue_4) :`true` (`/Game/CardStuff/SINGLEPLAYER/BP_Generator_Path.BranchRightPoint` _returnvalue_4)))
          (`KismetArrayLibrary.Array_Add` (`self.SpawnPoints`) (`SceneComponent.K2_GetComponentToWorld` _returnvalue_5))
          (`KismetArrayLibrary.Array_Add` (`self.SpawnPointVectors`) (`SceneComponent.GetForwardVector` _returnvalue_5))
          (`/Engine/EditorBlueprintResources/StandardMacros.DecrementInt` (`self.BranchesToSpawn#`)
            (:`  `
              _)))
        (if (== (`local.LoopIndex`) (`local.HallLength`))
          (bind _returnvalue_6 (`GameplayStatics.GetActorOfClass` "/Game/CardStuff/SINGLEPLAYER/BP_BlockGrid.BP_BlockGrid_C"))
          (`KismetArrayLibrary.Array_Add` (`/Game/CardStuff/SINGLEPLAYER/BP_BlockGrid.EndPoints` _returnvalue_6) (`KismetMathLibrary.MakeTransform` (`KismetMathLibrary.MakeVector` (`KismetMathLibrary.Conv_IntToDouble` (* (/ _returnvalue_x 100) 100)) (`KismetMathLibrary.Conv_IntToDouble` (* (/ _returnvalue_y 100) 100)) _returnvalue_z) _returnvalue_rotation)))))))

(fn `UserConstructionScript`)