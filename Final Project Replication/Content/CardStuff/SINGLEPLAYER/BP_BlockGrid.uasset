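; BP_BlockGrid is an actor that spawns rooms at BeginPlay and fills the open cells around them with block instances.
; It spawns a start room above its origin, then a standard room at each EndPoints transform.
; It then line-traces down over a square grid centered on world origin, adding hierarchical instanced mesh blocks where nothing is hit.
; The hit-tag switch has no cases, and the mesh add/remove functions are stubs.
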(event `self.ReceiveBeginPlay`
  (bind _returnvalue (`SceneComponent.GetRelativeTransform` (`self.DefaultSceneRoot`)))
  (`|SpawnActorFromClass` "/Game/CardStuff/SINGLEPLAYER/BP_Start_Room.BP_Start_Room_C" (`KismetMathLibrary.MakeTransform` (`KismetMathLibrary.MakeVector` (.x (.location _returnvalue)) (.y (.location _returnvalue)) 250.0) (`KismetMathLibrary.MakeRotator` 0.0)) "Undefined" "MultiplyWithRoot" null null)
  (`|ExecutionSequence`
    (:`then_0`
      (for _array_element (`self.EndPoints`)
        (`KismetSystemLibrary.PrintString` (`KismetStringLibrary.Conv_TransformToString` _array_element))
        (`|SpawnActorFromClass` "/Game/CardStuff/SINGLEPLAYER/BP_Standard_Room.BP_Standard_Room_C" _array_element "AlwaysSpawn" "MultiplyWithRoot" null null)))
    (:`then_1`
      (for _index (range -50 51)
        (for _index_2 (range -50 51)
          (bind (_coordinatesout _locationout) (`self.IntPoint-Location` (make `IntPoint` _index _index_2)))
          (bind _output_get (set `self.GridLocation` _locationout))
          (bind _outhit (`KismetSystemLibrary.LineTraceSingle` (`KismetMathLibrary.MakeVector` (.x _output_get) (.y _output_get) (+ (.z _output_get) 500.0)) (`KismetMathLibrary.MakeVector` (.x _output_get) (.y _output_get) (- (.z _output_get) -10.0)) "TraceTypeQuery1" true))
          (if (`GameplayStatics.BreakHitResult` _outhit)
            (switch `name` (`|GetArrayItem` (`Actor.Tags` (`.HitActor` (`GameplayStatics.BreakHitResult` _outhit)))))
            (else
              (`InstancedStaticMeshComponent.AddInstance` (`self.HierarchicalInstancedStaticMesh`) (`KismetMathLibrary.MakeTransform` (`self.GridLocation`)) false))))))))

(fn `AddNewMeshInstance`
  (params (Mesh :type "StaticMesh Object Reference") (Transform :type "Transform Structure"))
  (returns (`Successful?` :type Boolean) (Index :type Integer))
  (return false 0))

(fn `IntPoint-Location`
  (params (CoordinatesIn :type "IntPoint Structure") (LocationIn :type "Vector Structure"))
  (returns (CoordinatesOut :type "IntPoint Structure") (LocationOut :type "Vector Structure"))
  (bind _blocksize (`self.BlockSize`))
  (bind (_returnvalue_x _returnvalue_y) (break `IntPoint` (* CoordinatesIn (make `IntPoint` _blocksize _blocksize))))
  (bind (_returnvalue_x_2 _returnvalue_y_2) (`KismetMathLibrary.BreakVector` (/ LocationIn (`self.BlockSize`))))
  (return (make `IntPoint` (`KismetMathLibrary.FTrunc` _returnvalue_x_2) (`KismetMathLibrary.FTrunc` _returnvalue_y_2)) (`KismetMathLibrary.MakeVector` (`KismetMathLibrary.Conv_IntToDouble` _returnvalue_x) (`KismetMathLibrary.Conv_IntToDouble` _returnvalue_y))))

(fn `RemoveAllInstances`
  (returns (`Successful?` :type Boolean))
  (return false))

(fn `RemoveAllMeshInstances`
  (params (Mesh :type "StaticMesh Object Reference"))
  (returns (`Successful?` :type Boolean))
  (return false))

(fn `RemoveMeshInstance`
  (params (Mesh :type "StaticMesh Object Reference") (Index :type Integer))
  (returns (Successful :type Boolean))
  (return false))

(fn `UserConstructionScript`)