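; Single-player standard room actor with logic to procedurally generate winding, branching corridors.
; SpawnCorridor(s) chains BP_Generator_Path actors from each previous StartPoint, randomly varying yaw after the first piece.
; While BranchesToSpawn is positive, random or near-end pieces add side points to SpawnPoints, and each corridor's end is registered in BP_BlockGrid's EndPoints.
; The EventGraph loop seeding SpawnPoints from PathStartPoint is disconnected, so nothing here triggers generation.
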(event `self.ReceiveBeginPlay`)

(fn `SpawnCorridor(s)`
  (params (SpawnLoc :type "Transform Structure") (HallLength :type Integer))
  (locals (CorridorRotation :type "Rotator Structure" :default (struct)) (CorridorSpawnLoc :type "Transform Structure") (LoopIndex :type Integer) (NewSpawnPoint :type "SceneComponent Object Reference"))
  (bind _corridorspawnloc_location (`KismetMathLibrary.BreakTransform` (`local.CorridorSpawnLoc`)))
  (bind _newspawnpoint (`local.NewSpawnPoint`))
  (bind _corridorspawnloc (`local.CorridorSpawnLoc`))
  (bind (_returnvalue_location _returnvalue_rotation _returnvalue_scale) (`KismetMathLibrary.BreakTransform` (`SceneComponent.K2_GetComponentToWorld` _newspawnpoint)))
  (bind _returnvalue (> (`self.BranchesToSpawn#`) 0))
  (`KismetSystemLibrary.PrintString` (`KismetStringLibrary.Conv_IntToString` HallLength))
  (set `local.CorridorSpawnLoc` SpawnLoc)
  (for _index (range (+ HallLength 1))
    (set `local.LoopIndex` _index)
    (if (`self.First`)
      (set `local.CorridorRotation` (`KismetMathLibrary.MakeRotator` 0.0 0.0 (.yaw (.rotation _corridorspawnloc))))
      (set `self.First` false)
      (else
        (set `local.CorridorRotation` (`KismetMathLibrary.MakeRotator` 0.0 0.0 (+ (.yaw (.rotation _corridorspawnloc)) (`KismetMathLibrary.RandomFloatInRange` -45.0 45.0))))))
    (bind _returnvalue_2 (`|SpawnActorFromClass` "/Game/CardStuff/SINGLEPLAYER/BP_Generator_Path.BP_Generator_Path_C" (`KismetMathLibrary.MakeTransform` _corridorspawnloc_location (`local.CorridorRotation`)) "Undefined" "MultiplyWithRoot" null null))
    (bind _startpoint (`/Game/CardStuff/SINGLEPLAYER/BP_Generator_Path.StartPoint` _returnvalue_2))
    (set `local.NewSpawnPoint` _startpoint)
    (set `local.CorridorSpawnLoc` (`SceneComponent.K2_GetComponentToWorld` _startpoint))
    (if (or (and (> (`KismetMathLibrary.RandomFloat`) 0.9) _returnvalue) (and _returnvalue (== (`local.LoopIndex`) (- (`local.HallLength`) 1))))
      (`KismetArrayLibrary.Array_Add` (`self.SpawnPoints`) (`SceneComponent.K2_GetComponentToWorld` (select `bool` (`KismetMathLibrary.RandomBool`) :`false` (`/Game/CardStuff/SINGLEPLAYER/BP_Generator_Path.BranchLeftPoint` _returnvalue_2) :`true` (`/Game/CardStuff/SINGLEPLAYER/BP_Generator_Path.BranchRightPoint` _returnvalue_2)))))
    (if (== (`local.LoopIndex`) (`local.HallLength`))
      (bind _returnvalue_3 (`GameplayStatics.GetActorOfClass` "/Game/CardStuff/SINGLEPLAYER/BP_BlockGrid.BP_BlockGrid_C"))
      (`KismetArrayLibrary.Array_Add` (`/Game/CardStuff/SINGLEPLAYER/BP_BlockGrid.EndPoints` _returnvalue_3) (`KismetMathLibrary.MakeTransform` (+ (* (`SceneComponent.GetForwardVector` _newspawnpoint) 250.0) _returnvalue_location) _returnvalue_rotation _returnvalue_scale)))))

(fn `UserConstructionScript`)