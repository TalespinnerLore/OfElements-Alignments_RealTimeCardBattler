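; Game instance for the multiplayer card game that handles session failures and carries player data.
; Network and travel errors print the failure type in red and destroy the session; LeaveSession opens the menu level and destroys the session.
; StorePlayerData and LoadPlayerData copy stats, deck, passive deck and companion between the local BP_DeckBearer_Char and instance variables, so they can outlive level changes.
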(event `self.ReceiveInit`)

(event `self.ReceiveShutdown`)

(event `self.HandleNetworkError`
  (params (FailureType :type "ENetworkFailure Enum" :default "NetDriverAlreadyExists") (bIsServer :type Boolean))
  ;[1 1 1] Handle Network/Handle Errors.
  (`KismetSystemLibrary.PrintString` (`|GetEnumeratorNameAsString` FailureType) true true (struct :`R` 1.0 :`A` 1.0) 5.0)
  (`DestroySessionCallbackProxy.DestroySession` (`GameplayStatics.GetPlayerController` 0) :!label _label))

(event `self.HandleTravelError`
  (params (FailureType :type "ETravelFailure Enum" :default "NoLevel"))
  ;[1 1 1] Handle Network/Handle Errors.
  (`KismetSystemLibrary.PrintString` (`|GetEnumeratorNameAsString` FailureType) true true (struct :`R` 1.0 :`A` 1.0) 5.0)
  (goto _label))

(event `LeaveSession`
  ;[1 1 1] ResetSession
  (`GameplayStatics.OpenLevel` "MenuLevel")
  (`DestroySessionCallbackProxy.DestroySession` (`GameplayStatics.GetPlayerController` 0)))

(fn `LoadPlayerData`
  (bind _asbp_deck_bearer_char (cast `/Game/CardStuff/PLAYER/BP_DeckBearer_Char` (`GameplayStatics.GetPlayerCharacter` 0)))
  (set `/Game/CardStuff/PLAYER/BP_DeckBearer_Char.PlayerStats` (`self.Playerstats`) _asbp_deck_bearer_char)
  (set `/Game/CardStuff/PLAYER/BP_DeckBearer_Char.PlayerDeck` (`self.Playerdeck`) _asbp_deck_bearer_char)
  (set `/Game/CardStuff/PLAYER/BP_DeckBearer_Char.PassiveDeck` (`self.playerpassives`) _asbp_deck_bearer_char)
  (set `/Game/CardStuff/PLAYER/BP_DeckBearer_Char.CompanionCard[Zone-Companion]` (`self.companion`) _asbp_deck_bearer_char))

(fn `StorePlayerData`
  (bind _asbp_deck_bearer_char (cast `/Game/CardStuff/PLAYER/BP_DeckBearer_Char` (`GameplayStatics.GetPlayerCharacter` 0)))
  (set `self.Playerstats` (`/Game/CardStuff/PLAYER/BP_DeckBearer_Char.PlayerStats` _asbp_deck_bearer_char))
  (set `self.Playerdeck` (`/Game/CardStuff/PLAYER/BP_DeckBearer_Char.PlayerDeck` _asbp_deck_bearer_char))
  (set `self.playerpassives` (`/Game/CardStuff/PLAYER/BP_DeckBearer_Char.PassiveDeck` _asbp_deck_bearer_char))
  (set `self.companion` (`/Game/CardStuff/PLAYER/BP_DeckBearer_Char.CompanionCard[Zone-Companion]` _asbp_deck_bearer_char)))