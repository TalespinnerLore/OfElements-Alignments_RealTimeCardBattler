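; BP_DeckbuildController is a player controller that sets up the deckbuilding, level-up and menu screens.
; BeginPlay feeds the deck bearer character's stats and decks into the widgets, showing only the main menu; Enter opens the menu in UI-only input.
; Save helpers load or overwrite existing slots; a missing slot gets a new save object that is never written.
; It also provides a cursor hit-location lookup and placeholder unit getters returning fixed defaults.
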(event `self.ReceiveBeginPlay`
  (bind _asbp_deck_bearer_char (cast `/Game/CardStuff/PLAYER/BP_DeckBearer_Char` (`GameplayStatics.GetPlayerCharacter` 0)))
  (bind _output_get (set `self.PlayerRef` _asbp_deck_bearer_char))
  (bind _returnvalue (`|CreateWidget` :`Class` "/Game/CardStuff/UI/DeckbuildingUI/WBP_Deckbuilding.WBP_Deckbuilding_C" :`OwningPlayer` self :`PlayerStats` (`/Game/CardStuff/PLAYER/BP_DeckBearer_Char.PlayerStats` _output_get) :`InitialPlayerDeck` (`/Game/CardStuff/PLAYER/BP_DeckBearer_Char.PlayerDeck` _output_get) :`InitialPlayerPassiveDeck` (`/Game/CardStuff/PLAYER/BP_DeckBearer_Char.PassiveDeck` _output_get)))
  (bind _output_get_2 (set `self.DeckBuildingScreen` _returnvalue))
  (set `Widget.Visibility` "Collapsed" _output_get_2)
  (`UserWidget.AddToViewport` _output_get_2 0)
  (set `self.bShowMouseCursor` true)
  (bind _returnvalue_2 (`|CreateWidget` "/Game/CardStuff/UI/DeckbuildingUI/WBP_LevelUP.WBP_LevelUP_C" null (`/Game/CardStuff/PLAYER/BP_DeckBearer_Char.PlayerStats` (`self.PlayerRef`))))
  (bind _output_get_3 (set `self.statscreen` _returnvalue_2))
  (`Widget.SetVisibility` _output_get_3 "Collapsed")
  (`UserWidget.AddToViewport` _returnvalue_2 0)
  (bind _returnvalue_3 (`|CreateWidget` "/Game/CardStuff/UI/DeckbuildingUI/WBP_Menu.WBP_Menu_C"))
  (bind _output_get_4 (set `self.Menu` _returnvalue_3))
  (`Widget.SetVisibility` _output_get_4 "Collapsed")
  (`UserWidget.AddToViewport` _returnvalue_3 0)
  (bind _returnvalue_4 (`|CreateWidget` "/Game/CardStuff/UI/DeckbuildingUI/WBP_MainMenuWIDGET.WBP_MainMenuWIDGET_C"))
  (`UserWidget.AddToViewport` _returnvalue_4 0))

(event `Key|Enter`
  (params (Key :type "Key Structure"))
  (:`Pressed`
    (set `Widget.Visibility` "Visible" (`self.Menu`))
    (`WidgetBlueprintLibrary.SetInputMode_UIOnlyEx` self null)))

(fn `ActorIsMoving`
  (returns (IsMoving :type Boolean))
  (return false))

(fn `GetAlignment`
  (returns (Alignment1 :type "/Game/CardStuff/ENUM_ST_DT/Enums/TypeAlignment_Enum Enum") (Alignment2 :type "/Game/CardStuff/ENUM_ST_DT/Enums/TypeAlignment_Enum Enum"))
  (return "NewEnumerator21" "NewEnumerator21"))

(fn `GetAttackRange`
  (returns (AttackRange :type "Float (double-precision)"))
  (return 0.0))

(fn `GetCommand`
  (returns (Command :type "/Game/CardStuff/ENUM_ST_DT/Enums/Command_Enum Enum"))
  (return "NewEnumerator0"))

(fn `GetCost`
  (returns (Cost :type Integer))
  (return 0))

(fn `GetElement`
  (returns (Elem1 :type "/Game/CardStuff/ENUM_ST_DT/Enums/ElementalAlignment_Enum Enum") (Elem2 :type "/Game/CardStuff/ENUM_ST_DT/Enums/ElementalAlignment_Enum Enum"))
  (return "NewEnumerator11" "NewEnumerator11"))

(fn `GetHP`
  (returns (CurrentHP :type Integer) (MaxHP :type Integer))
  (return 0 0))

(fn `GetLocationUnderCursor`
  (returns (Location :type "Vector Structure"))
  (return (`.Location` (`GameplayStatics.BreakHitResult` (`self.GetHitResultUnderCursorByChannel` "TraceTypeQuery1")))))

(fn `GetTeam`
  (returns (Team :type "/Game/CardStuff/ENUM_ST_DT/Enums/TeamID Enum"))
  (return "NewEnumerator4"))

(fn `LoadGameFromSlot`
  (params (SaveSlot :type String))
  (bind _returnvalue (`GameplayStatics.DoesSaveGameExist` SaveSlot))
  (if _returnvalue
    (bind _returnvalue_2 (`GameplayStatics.LoadGameFromSlot` (`local.SaveSlot`)))
    (set `self.SaveGame` _returnvalue_2)))

(fn `SaveGameToSlot`
  (params (SaveSlot :type String))
  (bind _returnvalue (`GameplayStatics.DoesSaveGameExist` SaveSlot))
  (if _returnvalue
    (`GameplayStatics.SaveGameToSlot` (`self.SaveGame`) (`local.SaveSlot`))
    (else
      (bind _returnvalue_2 (`GameplayStatics.CreateSaveGameObject` "/Game/CardStuff/PLAYER/SAVE_1.SAVE_1_C"))
      (set `self.SaveGame` _returnvalue_2)
      (set `/Game/CardStuff/PLAYER/SAVE_1.CurrentLevel_Name` (`KismetStringLibrary.Conv_StringToName` (`KismetSystemLibrary.GetObjectName` (`self.GetLevel`))) _returnvalue_2)
      (set `/Game/CardStuff/PLAYER/SAVE_1.SpawnLocation` (`self.K2_GetActorLocation` (`self.PlayerRef`)) _returnvalue_2))))

(fn `UserConstructionScript`)