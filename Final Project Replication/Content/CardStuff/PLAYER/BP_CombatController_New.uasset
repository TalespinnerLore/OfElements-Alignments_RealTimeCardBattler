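; Player controller for a card-driven unit-command game, combining RTS-style selection with a deck hand and two-element mana.
; Right-drag box-selects units through the HUD, and left-click sends them follow, attack or move commands via their AI controllers, based on the cursor trace.
; BeginPlay builds the hand UI from the character's stats and deck, while mana functions track reserved, unspent and spendable pools.
; Releasing left-click plays placeholder cards; several interface getters return fixed values.
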(event `CommandSelectedUnits`
  (bind (_hit _location _hit_actor _hitpawn) (`self.GetLocationUnderCursor`))
  (bind _selectedactor (`self.SelectedActor`))
  (bind _selectedactor_2 (`self.SelectedActor`))
  (bind _selectedactors (`/Game/CardStuff/UI/BP_TEstHUD.SelectedActors` (`self.PlayerHUD`)))
  ;[1 1 1] depending on clicked result: if self, selected units follow; if enemy, selected units attack, if ground, selected units move to point.
  (set `self.SelectedActor` _hit_actor)
  (set `self.SelectedLocation` _location)
  (if (== _hitpawn (`self.K2_GetPawn` self))
    (for _array_element _selectedactors
      (message `/Game/CardStuff/AI_UNITS/BPI_COMBAT.SetCommand` (`AIBlueprintHelperLibrary.GetAIController` _array_element) "NewEnumerator1" (0.0 0.0 0.0) _selectedactor)
      (`KismetSystemLibrary.PrintString` "follow")
      (set `/Game/BP_TestUnit_Auto2.IsSelected` false (cast `/Game/BP_TestUnit_Auto2` _array_element :!pure true)))
    (set `self.HasSelectedActors` false)
    (elif (and (not (`self.ActorHasTag` _selectedactor_2 (`KismetStringLibrary.Conv_StringToName` (`|GetEnumeratorNameAsString` (`self.TeamID`))))) (`self.ActorHasTag` _selectedactor_2 "unit"))
      (for _array_element_2 _selectedactors
        (message `/Game/CardStuff/AI_UNITS/BPI_COMBAT.SetCommand` (`AIBlueprintHelperLibrary.GetAIController` _array_element_2) "NewEnumerator3" (0.0 0.0 0.0) _selectedactor)
        (`KismetSystemLibrary.PrintString` "getem")
        (bind _asbp_test_unit (cast `/Game/BP_TestUnit_Auto2` _array_element_2 :!pure true))
        (set `/Game/BP_TestUnit_Auto2.IsSelected` false _asbp_test_unit)
        (set `/Game/BP_TestUnit_Auto2.AttackTarget` (`self.SelectedActor`) _asbp_test_unit))
      (set `self.HasSelectedActors` false)
      (else
        (for _array_element_3 _selectedactors
          (message `/Game/CardStuff/AI_UNITS/BPI_COMBAT.SetCommand` (`AIBlueprintHelperLibrary.GetAIController` _array_element_3) "NewEnumerator2" (`self.SelectedLocation`) null)
          (`KismetSystemLibrary.PrintString` "moveto")
          (set `/Game/BP_TestUnit_Auto2.IsSelected` false (cast `/Game/BP_TestUnit_Auto2` _array_element_3 :!pure true)))
        (set `self.HasSelectedActors` false)))))

(event `UpdateUnitToFollow`
  ;[1 1 1] Tell Selected Units to Follow/Roam
)

(event `Select`
  (bind (_hit _location _hit_actor) (`self.GetLocationUnderCursor`))
  (bind _selectedactors (`/Game/CardStuff/UI/BP_TEstHUD.SelectedActors` (`self.PlayerHUD`)))
  ;[1 1 1] Is Selected: CLICK - If player clicked, follow player; if enemy clicked, attack enemy; if location clicked, move to location
  (set `self.HasSelectedActors` false)
  (`/Engine/EditorBlueprintResources/StandardMacros.IsValid` _hit_actor
    (:`Is Valid`
      (if (== (`self.K2_GetPawn` self) _hit_actor)
        (for _array_element _selectedactors
          (`/Game/CardStuff/AI_UNITS/AIC_Enemy_Base.Set State as Obeying Player` (`/Game/BP_TestUnit_Auto2.AIC` (cast `/Game/BP_TestUnit_Auto2` _array_element :!pure true))))
        (elif (`self.ActorHasTag` _hit_actor (`KismetStringLibrary.Conv_StringToName` (`|GetEnumeratorNameAsString` (`self.TeamID`))))
          (for _array_element_2 _selectedactors
            (bind _asbp_test_unit (cast `/Game/BP_TestUnit_Auto2` _array_element_2 :!pure true))
            (bind _output_get (set `/Game/BP_TestUnit_Auto2.AttackTarget` _hit_actor _asbp_test_unit))
            (`/Game/CardStuff/AI_UNITS/AIC_Enemy_Base.Set State as Attacking` (`/Game/BP_TestUnit_Auto2.AIC` _asbp_test_unit) _output_get))
          (else
            (for _array_element_3 (`/Game/CardStuff/UI/BP_TEstHUD.SelectedActors` (`self.PlayerHUD`)) :!label _label
              (bind _asbp_test_unit_2 (cast `/Game/BP_TestUnit_Auto2` _array_element_3 :!pure true))
              (`/Game/CardStuff/AI_UNITS/AIC_Enemy_Base.SetPointOfInterest` (`/Game/BP_TestUnit_Auto2.AIC` _asbp_test_unit_2) _location)
              (set `/Game/BP_TestUnit_Auto2.IsBeingDirected` true _asbp_test_unit_2))))))
    (:`Is Not Valid`
      (goto _label))))

(event `UpdateUnitToPassiveRoam`
  ;[1 1 1] Tell Selected Units to Follow/Roam
)

(event `Key|RightMouseButton`
  (params (Key :type "Key Structure"))
  (bind _playerhud (`self.PlayerHUD`))
  (bind (_locationx _locationy) (`self.GetMousePosition` self))
  (bind _returnvalue (`KismetMathLibrary.MakeVector2D` _locationx _locationy))
  ;[1 1 1] Drag to draw select box
  (:`Pressed`
    (if (not (`self.HasSelectedActors`))
      (`/Game/CardStuff/UI/BP_TEstHUD.Event Draw Box` _playerhud true _returnvalue)
      (`KismetSystemLibrary.Delay` 0.2)
      (`self.CheckForSelectedActors`)))
  (:`Released`
    (if true
      (`/Game/CardStuff/UI/BP_TEstHUD.Event Draw Box` _playerhud false _returnvalue))))

(event `PauseMenu_Continue`
  ;[1 1 1] \toggle Pause Menu
  (bind _pausemenu (`self.PauseMenu`)
    (:`then`
      (if (`Widget.IsVisible` _pausemenu)
        (`Widget.SetVisibility` (`self.PauseMenu`) "Collapsed")
        (set `self.bShowMouseCursor` true)
        (`WidgetBlueprintLibrary.SetInputMode_GameAndUIEx` self null "DoNotLock" false)
        (else
          (`Widget.SetVisibility` (`self.PauseMenu`) "Visible")
          (set `self.bShowMouseCursor` true :!label _label_2)
          (`WidgetBlueprintLibrary.SetInputMode_UIOnlyEx` self (`self.PauseMenu`)))))
    (:`else`
      (bind _returnvalue (`|CreateWidget` "/Game/CardStuff/UI/MenuUI/WBP_GameMenu.WBP_GameMenu_C" self self))
      (bind _output_get (set `self.PauseMenu` _returnvalue))
      (`UserWidget.AddToViewport` _output_get 0)
      (goto _label_2))))

(event `Key|MiddleMouseButton`
  (params (Key :type "Key Structure"))
  (bind _selectedactors (`/Game/CardStuff/UI/BP_TEstHUD.SelectedActors` (`self.PlayerHUD`)))
  ;[1 1 1] clear selected actors
  (:`Pressed`
    (`KismetSystemLibrary.PrintString` "reset selected")
    (for _array_element _selectedactors
      (`/Game/CardStuff/UI/BP_TEstHUD.SetHighlight` (`self.PlayerHUD`) false _array_element))
    (`KismetArrayLibrary.Array_Clear` _selectedactors)
    (set `self.HasSelectedActors` false)))

(event `Key|LeftMouseButton`
  (params (Key :type "Key Structure"))
  ;[1 1 1] Spawn Actor at Placeholder
  (:`Pressed`
    (if (`self.HasSelectedActors`)
      (`self.CommandSelectedUnits`)
      (else
        (`KismetSystemLibrary.PrintString` "command")
        (`KismetSystemLibrary.PrintString` (`KismetSystemLibrary.GetDisplayName` (`.Hit Actor` (`self.GetLocationUnderCursor`)))))))
  (:`Released`
    (if (`self.Placing`)
      (`/Game/CardStuff/UI/CombatUI/WBP_CardInHand.PlaceThing` (`/Game/CardStuff/AI_UNITS/BP_Placeholder.OriginCard` (`self.Placeholder`))))))

(event `self.ReceiveBeginPlay`
  (bind _returnvalue (subsystem `EnhancedInputLocalPlayerSubsystem`))
  ;[1 1 1] Initialize Values and references
  (`/Engine/EditorBlueprintResources/StandardMacros.IsValid` _returnvalue
    (:`Is Valid`
      (`EnhancedInputSubsystemInterface.AddMappingContext` _returnvalue null 0 (struct))
      (set `self.PlayerHUD` (cast `/Game/CardStuff/UI/BP_TEstHUD` (`self.GetHUD`) :!pure true))
      (set `self.bShowMouseCursor` true)
      (bind _asbp_deck_bearer_char (cast `/Game/CardStuff/PLAYER/BP_DeckBearer_Char` (`GameplayStatics.GetPlayerCharacter` 0)))
      (set `self.PlayerRef` _asbp_deck_bearer_char)
      (bind _returnvalue_2 (`|CreateWidget` "/Game/CardStuff/UI/CombatUI/WBP_Hand.WBP_Hand_C"))
      (bind _output_get (set `self.Mana+HandUI` _returnvalue_2))
      (`UserWidget.AddToViewport` _output_get 0)
      (`self.SetStats`)
      (`/Game/CardStuff/PLAYER/BP_DeckBearer_Char.ShuffleDeck` (`self.PlayerRef`))
      (`self.Draw New Hand`))))

(event `Key|LeftShift`
  (params (Key :type "Key Structure"))
  ;[1 1 1] damage testing
  (:`Pressed`
    (bind _outactors (`GameplayStatics.GetAllActorsOfClass` "/Game/BP_TestUnit_Auto2.BP_TestUnit_C"))
    (for _array_element _outactors
      (`GameplayStatics.ApplyDamage` _array_element 1.0))))

(event `/Game/CardStuff/AI_UNITS/BPI_COMBAT.AttackTargetActor`
  (params (EnemyActor :type "Actor Object Reference"))
  ;[1 0.7942 0] Interface Functions
  (`GameplayStatics.ApplyDamage` EnemyActor (`.Attack_4_E0667AAF434743A13F0B8E8BBB7B487A` (break `/Game/CardStuff/ENUM_ST_DT/Structs/ST_CreatureStats` (`.CombatStats_72_E3CFF4DF49D2C218E94803A56B5BA109` (break `/Game/CardStuff/ENUM_ST_DT/Structs/PlayerStats_Struct` (`/Game/CardStuff/PLAYER/BP_DeckBearer_Char.PlayerStats` (`self.PlayerRef`))))))))

(event `/Game/CardStuff/AI_UNITS/BPI_COMBAT.UnReserveMana`
  (params (Cost :type Integer) (Elem1 :type "/Game/CardStuff/ENUM_ST_DT/Enums/ElementalAlignment_Enum Enum" :default "NewEnumerator11") (Elem2 :type "/Game/CardStuff/ENUM_ST_DT/Enums/ElementalAlignment_Enum Enum" :default "NewEnumerator11"))
  ;[1 0.7942 0] Interface Functions
  (`self.Unreserve_Mana` Cost Elem1 Elem2))

(fn `ActorIsMoving`
  (returns (IsMoving :type Boolean))
  (return (`self.Moving`)))

(fn `ChangeReserved`
  (params (PrimaryAddedReservedMana :type Integer) (SecondaryAddedReservedMana :type Integer))
  (set `self.ReservedMana#1` (+ PrimaryAddedReservedMana (`self.ReservedMana#1`)))
  (set `self.ReservedMana#2` (+ SecondaryAddedReservedMana (`self.ReservedMana#2`)))
  (`/Game/CardStuff/UI/CombatUI/WBP_ManaBAr.ChangeValues` (`/Game/CardStuff/UI/CombatUI/WBP_Hand.WBP_ManaBar1` (`self.Mana+HandUI`)) (`self.ReservedMana#1`) (`self.UnspentMana#1`))
  (`/Game/CardStuff/UI/CombatUI/WBP_ManaBAr.ChangeValues` (`/Game/CardStuff/UI/CombatUI/WBP_Hand.WBP_ManaBar2` (`self.Mana+HandUI`)) (`self.ReservedMana#2`) (`self.UnspentMana#2`))
  (`self.SetSpendableMana`))

(fn `ChangeSpendable`
  (params (PrimaryNewlySpentMana :type Integer) (SecondaryNewlySpentMana :type Integer))
  (bind _unspentmana_2 (`self.UnspentMana#2`))
  (set `self.UnspentMana#1` (- (`self.UnspentMana#1`) PrimaryNewlySpentMana))
  (set `self.UnspentMana#2` (- _unspentmana_2 SecondaryNewlySpentMana))
  (`KismetSystemLibrary.PrintString` (`KismetStringLibrary.Concat_StrStr` "Unspent: " (`KismetStringLibrary.Conv_IntToString` _unspentmana_2) " \nNewlySpent: " (`KismetStringLibrary.Conv_IntToString` SecondaryNewlySpentMana)) true true (struct :`R` 1.0 :`B` 0.968575 :`A` 1.0) 10.0)
  (`/Game/CardStuff/UI/CombatUI/WBP_ManaBAr.ChangeValues` (`/Game/CardStuff/UI/CombatUI/WBP_Hand.WBP_ManaBar1` (`self.Mana+HandUI`)) (`self.ReservedMana#1`) (`self.UnspentMana#1`))
  (`/Game/CardStuff/UI/CombatUI/WBP_ManaBAr.ChangeValues` (`/Game/CardStuff/UI/CombatUI/WBP_Hand.WBP_ManaBar2` (`self.Mana+HandUI`)) (`self.ReservedMana#2`) (`self.UnspentMana#2`))
  (`self.SetSpendableMana`))

(fn `CheckForSelectedActors`
  (set `self.HasSelectedActors` (> (`KismetArrayLibrary.Array_Length` (`/Game/CardStuff/UI/BP_TEstHUD.SelectedActors` (`self.PlayerHUD`))) 0)))

(fn `CheckResoucePastMax`
  (if (> (`self.UnspentMana#1`) (`self.MaxMana#1`))
    (set `self.UnspentMana#1` (`self.MaxMana#1`)))
  (if (> (`self.UnspentMana#2`) (`self.MaxMana#2`))
    (set `self.UnspentMana#2` (`self.MaxMana#2`))))

(fn `DefaultAttack`
  (params (TargetActor :type "Actor Object Reference"))
  (`|SpawnActorFromClass` "/Game/CardStuff/AI_UNITS/BP_AttackProjectile.BP_AttackProjectile_C" (`KismetMathLibrary.Conv_VectorToTransform` (`self.K2_GetActorLocation`)) "Undefined" "MultiplyWithRoot" null (`self.TeamID`) null (`KismetMathLibrary.SelectVector` (`self.K2_GetActorLocation` TargetActor) (`.Location` (`self.GetLocationUnderCursor`)) (`KismetSystemLibrary.IsValid` TargetActor)) null null))

(fn `Draw New Hand`
  (locals (TempArray :type "Array of /Game/CardStuff/ENUM_ST_DT/Structs/AllCardStats_Struct Structure"))
  (bind _playerref (`self.PlayerRef`))
  (bind _hand_zone_hand_ (`/Game/CardStuff/PLAYER/BP_DeckBearer_Char.Hand[Zone-Hand]` (`self.PlayerRef`)))
  (bind _returnvalue (`KismetArrayLibrary.Array_Length` _hand_zone_hand_))
  (bind _output_get (set `local.TempArray` _hand_zone_hand_))
  (if (> _returnvalue 0)
    (for _array_element _output_get
      (`/Game/CardStuff/PLAYER/BP_DeckBearer_Char.HandToDeck[Bottom]` _playerref _array_element)
      (`KismetSystemLibrary.PrintString` (`KismetStringLibrary.Conv_NameToString` (`.Name_88_7D4C302E4BEF2740318D68BD7176F70D` (break `/Game/CardStuff/ENUM_ST_DT/Structs/AllCardStats_Struct` _array_element))) true true (struct :`G` 0.212814 :`B` 1.0 :`A` 1.0) 10.0)))
  (`KismetSystemLibrary.PrintString` (`KismetStringLibrary.Concat_StrStr` "Hand size empty: " (`KismetStringLibrary.Conv_IntToString` _returnvalue)) true true (struct :`R` 0.963065 :`B` 1.0 :`A` 1.0) 10.0)
  (bind _newcards (`/Game/CardStuff/PLAYER/BP_DeckBearer_Char.DeckToHand[Draw]` _playerref (`self.MaxHandSize`)))
  (for _array_element_2 _newcards
    (bind _returnvalue_2 (`|CreateWidget` "/Game/CardStuff/UI/CombatUI/WBP_CardInHand.WBP_CardInHand_C" null _array_element_2 (`self.Mana+HandUI`) self))
    (`PanelWidget.AddChild` (`/Game/CardStuff/UI/CombatUI/WBP_Hand.HandBox` (`self.Mana+HandUI`)) _returnvalue_2)))

(fn `GetAlignment`
  (returns (Alignment1 :type "/Game/CardStuff/ENUM_ST_DT/Enums/TypeAlignment_Enum Enum") (Alignment2 :type "/Game/CardStuff/ENUM_ST_DT/Enums/TypeAlignment_Enum Enum"))
  (return "NewEnumerator21" "NewEnumerator21"))

(fn `GetAttackRange`
  (returns (AttackRange :type "Float (double-precision)"))
  (return (select `/Game/CardStuff/ENUM_ST_DT/Enums/AttackRange_Enum` (`self.Range`) :`NewEnumerator0` 200.0 :`NewEnumerator1` 400.0 :`NewEnumerator2` 600.0)))

(fn `GetCommand`
  (returns (Command :type "/Game/CardStuff/ENUM_ST_DT/Enums/Command_Enum Enum"))
  (return "NewEnumerator0"))

(fn `GetCost`
  (returns (Cost :type Integer))
  (return 0))

(fn `GetElement`
  (returns (Elem1 :type "/Game/CardStuff/ENUM_ST_DT/Enums/ElementalAlignment_Enum Enum") (Elem2 :type "/Game/CardStuff/ENUM_ST_DT/Enums/ElementalAlignment_Enum Enum"))
  (return "NewEnumerator11" "NewEnumerator11"))

(fn `GetHP`
  (returns (CurrentHP :type Integer) (MaxHP :type Integer))
  (return 0 0))

(fn `GetLocationUnderCursor`
  (returns (Hit :type Boolean) (Location :type "Vector Structure") (`Hit Actor` :type "Actor Object Reference") (HitPawn :type "Actor Object Reference"))
  (bind (_bblockinghit _binitialoverlap _time _distance _location _impactpoint _normal _impactnormal _physmat _hitactor) (`GameplayStatics.BreakHitResult` (`self.GetHitResultUnderCursorByChannel` "TraceTypeQuery1")))
  (return _bblockinghit _location _hitactor (`.HitActor` (`GameplayStatics.BreakHitResult` (`self.GetHitResultUnderCursorForObjects` (`|MakeArray` "ObjectTypeQuery3" :!type "EObjectTypeQuery Enum"))))))

(fn `GetTeam`
  (returns (Team :type "/Game/CardStuff/ENUM_ST_DT/Enums/TeamID Enum"))
  (return "NewEnumerator4"))

(fn `RefreshHand`
  (bind _playerref (`self.PlayerRef`))
  (`PanelWidget.ClearChildren` (`/Game/CardStuff/UI/CombatUI/WBP_Hand.HandBox` (`self.Mana+HandUI`)))
  (for _array_element (`/Game/CardStuff/PLAYER/BP_DeckBearer_Char.Hand[Zone-Hand]` (`self.PlayerRef`))
    (`/Game/CardStuff/PLAYER/BP_DeckBearer_Char.FieldToDeck[Bottom]` _playerref _array_element))
  (`/Game/CardStuff/PLAYER/BP_DeckBearer_Char.DeckToHand[Draw]` _playerref (`self.MaxHandSize`))
  (set `self.UnspentMana#1` (`self.MaxMana#1`))
  (set `self.UnspentMana#2` (`self.MaxMana#2`))
  (`self.ChangeSpendable` 0))

(fn `ResetSpendableMana`
  (set `self.UnspentMana#1` (`self.MaxMana#1`))
  (set `self.UnspentMana#2` (`self.MaxMana#2`))
  (`self.SetSpendableMana`)
  (`self.ChangeSpendable` 0))

(fn `SetSpendableMana`
  (set `self.SpendableMana#1` (- (`self.UnspentMana#1`) (`self.ReservedMana#1`)))
  (set `self.SpendableMana#2` (- (`self.UnspentMana#2`) (`self.ReservedMana#2`))))

(fn `SetStats`
  (locals (NewLocalVar :type "Float (double-precision)"))
  (bind (_name _level _perk1 _park2 _flaw _playeralignment _playerelem1 _playerelem2 _primaryalignment _secondaryalignment _mana _maximumdecksize _minimumdecksize _passiveslots _maximumhandsize _handrefreshrate _unittimeoutrate _leveledstats _combatstats) (break `/Game/CardStuff/ENUM_ST_DT/Structs/PlayerStats_Struct` (`/Game/CardStuff/PLAYER/BP_DeckBearer_Char.PlayerStats` (`self.PlayerRef`))))
  (bind (_primaryelement _secondaryelement _primarymana _pirmaryreservedmana _secondarymana _secondaryreservedmana) (break `/Game/CardStuff/ENUM_ST_DT/Structs/PlayerManaStruct` _mana))
  (`|ExecutionSequence`
    (:`then_0`
      (set `self.Alignment1` _primaryalignment)
      (set `self.Alignment2` _secondaryalignment)
      (set `self.MaxHandSize` _maximumhandsize))
    (:`then_1`
      (set `self.Element1` _primaryelement)
      (bind _output_get (set `self.Element2` _secondaryelement))
      (set `self.MaxMana#1` _primarymana)
      (set `self.ReservedMana#1` _pirmaryreservedmana)
      (if (`|EnumInequality` _output_get "NewEnumerator11")
        _
        (else
          _))
      (set `self.MaxMana#2` _secondarymana)
      (set `self.ReservedMana#2` _secondaryreservedmana)
      (set `self.UnspentMana#1` (`self.MaxMana#1`))
      (set `self.UnspentMana#2` (`self.MaxMana#2`))
      (`self.SetSpendableMana`)
      (`/Game/CardStuff/UI/CombatUI/WBP_ManaBAr.SetInitalValues` (`/Game/CardStuff/UI/CombatUI/WBP_Hand.WBP_ManaBar1` (`self.Mana+HandUI`)) (`self.ReservedMana#1`) (`self.MaxMana#1`) (`self.Element1`))
      (`/Game/CardStuff/UI/CombatUI/WBP_ManaBAr.SetInitalValues` (`/Game/CardStuff/UI/CombatUI/WBP_Hand.WBP_ManaBar2` (`self.Mana+HandUI`)) (`self.ReservedMana#2`) (`self.MaxMana#2`) (`self.Element2`))
      (set `self.Combat Stats` _combatstats))
    (:`then_2`
      (set `self.Hand Refresh Rate` _handrefreshrate)
      (set `self.Unit Timeout Rate` _unittimeoutrate))))

(fn `Unreserve_Mana`
  (params (A :type Integer) (A2 :type "/Game/CardStuff/ENUM_ST_DT/Enums/ElementalAlignment_Enum Enum" :default "NewEnumerator11") (B :type "/Game/CardStuff/ENUM_ST_DT/Enums/ElementalAlignment_Enum Enum" :default "NewEnumerator11"))
  (locals (ManaCost :type Integer) (PrimaryCost :type Integer) (SecondaryCost :type Integer))
  (bind _returnvalue (`|EnumEquality` A2 (`self.Element1`)))
  (bind _returnvalue_2 (* (`local.ManaCost`) -1))
  (bind _returnvalue_3 (/ (`local.ManaCost`) 2))
  (bind _returnvalue_4 (`KismetMathLibrary.Round` (+ _returnvalue_3 0.5)))
  (bind _returnvalue_5 (`KismetMathLibrary.Round` (- _returnvalue_3 0.5)))
  (set `local.ManaCost` A)
  (if (`|EnumEquality` "NewEnumerator11" B)
    (if _returnvalue
      (`self.ChangeReserved` _returnvalue_2)
      (else
        (`self.ChangeReserved` 0 _returnvalue_2)))
    (else
      (if _returnvalue
        (set `local.PrimaryCost` _returnvalue_4)
        (set `local.SecondaryCost` _returnvalue_5)
        (else
          (set `local.PrimaryCost` _returnvalue_5)
          (set `local.SecondaryCost` _returnvalue_4)))
      (`self.ChangeReserved` (* (`local.PrimaryCost`) -1) (* (`local.SecondaryCost`) -1)))))

(fn `UserConstructionScript`)